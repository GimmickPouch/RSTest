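; FloorTile is an environment actor that can be raised or lowered by animating its Z scale.
; LiftUp stores a target Z scale and sets a LiftingUp flag.
; While the flag is set, Tick moves the Z scale toward the target at a constant RaiseSpeed using FInterpToConstant, leaving X and Y unchanged, then clears the flag once the target is nearly reached.
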(event EventBeginPlay)

(event Collision|EventActorBeginOverlap
  (params (OtherActor :type Actor%20Object%20Reference)))

(event EventTick
  (params (DeltaSeconds :type Float%20%28single-precision%29))
  (bind _returnvalue (Transformation|GetActorScale3D))
  (bind (_x _y _z) (Math|Vector|BreakVector _returnvalue))
  (if (Variables|Default|GetLiftingUp)
    (Transformation|SetActorScale3D (Math|Vector|MakeVector _x _y (Math|Interpolation|FInterptoConstant _z (Variables|Default|GetLiftToZScale) (Utilities|Time|GetWorldDeltaSeconds) (Variables|Default|GetRaiseSpeed))))
    (if (Math|Float|NearlyEqual(Float) _z (Variables|Default|GetLiftToZScale) 1e-06)
      (Variables|Default|SetLiftingUp false))))

(fn ConstructionScript)

(fn LiftUp
  (params (LiftZScale :type Float%20%28single-precision%29))
  (Variables|Default|SetLiftToZScale LiftZScale)
  (Variables|Default|SetLiftingUp true))